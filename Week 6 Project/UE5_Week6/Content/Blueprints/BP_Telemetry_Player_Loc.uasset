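; Telemetry actor that records the player character's world location for export to a spreadsheet file.
; Every Tick it appends the first player's X, Y and Z as a comma-separated line to a growing text array.
; On EndPlay it writes the whole array to Player_Location.csv in the project directory, overwriting any previous file.
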(event EventBeginPlay)

(event Collision|EventActorBeginOverlap
  (params (OtherActor :type Actor%20Object%20Reference)))

(event EventTick
  (params (DeltaSeconds :type Float%20%28single-precision%29))
  (bind _returnvalue (Game|GetPlayerCharacter 0))
  (bind _returnvalue_2 (Transformation|GetActorLocation _returnvalue))
  ;[1 1 1] Log player location in SpreadSheet
  (Utilities|Array|Add (Variables|Default|GetSave%20Text) (Utilities|String|Append (Utilities|String|ToString(Float) (.x _returnvalue_2)) "," (Utilities|String|ToString(Float) (.y _returnvalue_2)) "," (Utilities|String|ToString(Float) (.z _returnvalue_2)))))

(event EventEndPlay
  (params (EndPlayReason :type EEndPlayReason%20Enum :default "Destroyed"))
  (Class|PFILib|SaveArrayText (Class|KismetSystemLibrary|GetProjectDirectory) "Player_Location.csv" (Variables|Default|GetSave%20Text) true))

(fn ConstructionScript)