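; BP_Door is a locked door that the player opens with the Interact key by spending a held key.
; Box overlap with the ThirdPersonCharacter sets whether interaction is allowed.
; A successful interaction decrements the character's key count and plays a timeline that drives the door's yaw, leaving it open.
; Without a key, a DoOnce-guarded UI_KeyRequired widget shows briefly, and the guard resets after its removal.
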(event OnComponentBeginOverlap(Box)
  (params (OverlappedComponent :type Primitive%20Component%20Object%20Reference) (OtherActor :type Actor%20Object%20Reference) (OtherComp :type Primitive%20Component%20Object%20Reference) (OtherBodyIndex :type Integer) (bFromSweep :type Boolean) (SweepResult :type Hit%20Result%20Structure%20%28by%20ref%29))
  ;[0 0 0] When player enters / leaves the collision box component we set the Boolean variable "Can Be Interacted With?" to true/false.
  (Utilities|Casting|CastToThirdPersonCharacter OtherActor)
  (Variables|Default|SetCan%20Be%20Interacted%20With? true))

(event OnComponentEndOverlap(Box)
  (params (OverlappedComponent :type Primitive%20Component%20Object%20Reference) (OtherActor :type Actor%20Object%20Reference) (OtherComp :type Primitive%20Component%20Object%20Reference) (OtherBodyIndex :type Integer))
  ;[0 0 0] When player enters / leaves the collision box component we set the Boolean variable "Can Be Interacted With?" to true/false.
  (Utilities|Casting|CastToThirdPersonCharacter OtherActor)
  (Variables|Default|SetCan%20Be%20Interacted%20With? false))

(event Custom|Open%20Door
  ;[0 0 0] This event will make the door open using a timeline
  (bind _door_angle (Timeline|Door%20TL Play)
    (:Update
      (Transformation|SetRelativeRotation (Variables|Default|GetDoor) (Math|Rotator|MakeRotator 0.0 0.0 _door_angle) false false))))

(event Input|ActionEvents|InputActionInteractKey
  (params (Key :type Key%20Structure :default "None"))
  ;[0.15 0.15 0.15 0.5] Open Door if the player has a key, otherwise display key required widget
  (:Pressed
    (if (and (Variables|Default|GetCan%20Be%20Interacted%20With?) (not (Variables|Default|GetDoor%20Open?)))
      (bind _asthird_person_character (Utilities|Casting|CastToThirdPersonCharacter (Game|GetPlayerCharacter 0)))
      (if (> (Variables|/Game/ThirdPersonBP/Blueprints/ThirdPersonCharacter.ThirdPersonCharacter_C|GetNumber%20Of%20Keys%20Held _asthird_person_character) 0)
        (Math|Integer|DecrementInt (Variables|/Game/ThirdPersonBP/Blueprints/ThirdPersonCharacter.ThirdPersonCharacter_C|GetNumber%20Of%20Keys%20Held _asthird_person_character)
          (:%20%20
            (CallFunction|OpenDoor)
            (Variables|Default|SetDoor%20Open? true)))
        (else
          (Utilities|FlowControl|DoOnce false :!label _label
            (:Completed
              (bind _returnvalue (UserInterface|CreateWidget "/Game/UI/UI_KeyRequired.UI_KeyRequired_C"))
              (UserInterface|Viewport|AddtoViewport _returnvalue 0)
              (Utilities|FlowControl|Delay 2.0)
              (Widget|RemovefromParent _returnvalue)
              (goto _label Reset))))))))

(fn ConstructionScript)