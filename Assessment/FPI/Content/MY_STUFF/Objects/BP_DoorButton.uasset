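; BP_DoorButton is an interactable button that opens a referenced door once, then disables itself and shows an activated material.
; It can start locked, swapping to a locked material on BeginPlay.
; Interacting while locked checks the first-person character for keys and, if any are held, unlocks the button and consumes one key, so opening takes another interaction.
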(event EventBeginPlay
  ;[0.15 0.15 0.15 0.5] Update texture to locked on spawn if door is locked
  (if (Variables|Default|GetLocked)
    (CallFunction|Lock)))

(event Collision|EventActorBeginOverlap
  (params (OtherActor :type Actor%20Object%20Reference)))

(event EventTick
  (params (DeltaSeconds :type Float%20%28single-precision%29)))

(event EventOnInteract
  ;[0.15 0.15 0.15 0.5] Open door when button pressed
  (bind _can_interact (CallFunction|IsInteractable))
  (if _can_interact
    (if (not (Variables|Default|GetLocked))
      (Class|SlidingDoor|OpenDoor (Variables|Default|GetDoorRef))
      (Variables|Default|Setinteractable false)
      (Rendering|Material|SetMaterial (Variables|Default|GetbuttonMesh) 0 "/Game/MY_STUFF/Materials/ButtonActivated_MAT.ButtonActivated_MAT")
      (else
        (bind _returnvalue (Actor|GetActorOfClass "/Game/FirstPerson/Blueprints/BP_FirstPersonCharacter.BP_FirstPersonCharacter_C"))
        (bind _haskeys (Default|IsPlayerHoldingKeys _returnvalue))
        (if _haskeys
          (CallFunction|Unlock)
          (Default|AlterNumKeys _returnvalue -1))))))

(fn ConstructionScript)

(fn Lock
  (Variables|Default|SetLocked true)
  (Rendering|Material|SetMaterial (Variables|Default|GetbuttonMesh) 0 "/Game/MY_STUFF/Materials/ButtonLocked_MAT.ButtonLocked_MAT"))

(fn Unlock
  (Variables|Default|SetLocked false)
  (Rendering|Material|SetMaterial (Variables|Default|GetbuttonMesh) 0 "/Game/MY_STUFF/Materials/Button_MAT.Button_MAT"))

(fn IsInteractable
  (return (Variables|Default|Getinteractable)))