(event EventOnInteract
  (bind _asui_end_screen (Utilities|Casting|CastToUI_EndScreen (Variables|Default|GetUI_Ref)))
  (Default|ShowEndScreen _asui_end_screen)
  (bind _returnvalue (Actor|GetActorOfClass "/Game/FirstPerson/Blueprints/BP_FirstPersonCharacter.BP_FirstPersonCharacter_C"))
  (Default|SetinMenuState _returnvalue true)
  (bind _returnvalue_2 (Actor|GetActorOfClass "/Game/MY_STUFF/Blueprints/BP_ObjectiveManager.BP_ObjectiveManager_C"))
  (Default|ChangeObjective _returnvalue_2 "YouWin" "YouWin"))

(event EventBeginPlay
  (bind _returnvalue (UserInterface|CreateWidget "/Game/MY_STUFF/UI/UI_EndScreen.UI_EndScreen_C"))
  (bind _output_get (Variables|Default|SetUI_Ref _returnvalue))
  (UserInterface|Viewport|AddtoViewport _output_get 0))

(fn ConstructionScript)

(fn IsInteractable
  (return (Variables|Default|GetisInteractable)))