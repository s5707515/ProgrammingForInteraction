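; BP_DoorButton is an interactable button that opens its linked door, optionally starting locked.
; On interact it opens DoorRef once and shows an activated material, or, if locked, spends one of the first-person character's keys to unlock, requiring another press to open.
; Lock and Unlock swap the button material, and sounds signal each outcome.
; The first interaction, successful or not, also updates the objective through BP_ObjectiveManager's UI.
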(event EventBeginPlay
  ;[0.15 0.15 0.15 0.5] Update texture to locked on spawn if door is locked
  (if (Variables|Default|GetLocked)
    (CallFunction|Lock)))

(event Collision|EventActorBeginOverlap
  (params (OtherActor :type Actor%20Object%20Reference)))

(event EventTick
  (params (DeltaSeconds :type Float%20%28single-precision%29)))

(event EventOnInteract
  ;[0.15 0.15 0.15 0.5] Open door when button pressed
  (Utilities|FlowControl|Sequence
    (:then_0
      (bind _can_interact (CallFunction|IsInteractable))
      (if _can_interact
        (if (not (Variables|Default|GetLocked))
          (Class|SlidingDoor|OpenDoor (Variables|Default|GetDoorRef))
          (Variables|Default|Setinteractable false)
          (Rendering|Material|SetMaterial (Variables|Default|GetbuttonMesh) 0 "/Game/MY_STUFF/Materials/ButtonActivated_MAT.ButtonActivated_MAT")
          (Audio|PlaySound2D "/Game/MY_STUFF/SFXs/ding_deep.ding_deep" 1.0 1.0 0.0 0 0)
          (else
            (bind _returnvalue (Actor|GetActorOfClass "/Game/FirstPerson/Blueprints/BP_FirstPersonCharacter.BP_FirstPersonCharacter_C"))
            (bind _haskeys (Default|IsPlayerHoldingKeys _returnvalue))
            (if _haskeys
              (CallFunction|Unlock)
              (Default|AlterNumKeys _returnvalue -1)
              (Audio|PlaySound2D "/Game/MY_STUFF/SFXs/click.click" 1.0 1.0 0.0 0 0)
              (else
                (Audio|PlaySound2D "/Game/MY_STUFF/SFXs/negative_2.negative_2" 1.0 1.0 0.0 0 0)))))))
    (:then_1
      ;[0.15 0.15 0.15 0.5] Update Objective
      (if (Variables|Default|GetfirstInteract)
        (bind _returnvalue_2 (Actor|GetActorOfClass "/Game/MY_STUFF/Blueprints/BP_ObjectiveManager.BP_ObjectiveManager_C"))
        (Class|Objectives|ChangeObjective (Variables|/Game/MY_STUFF/Blueprints/BP_ObjectiveManager.BP_ObjectiveManager_C|GetUI_Ref _returnvalue_2) (Variables|Default|Getobjective))
        (Variables|Default|SetfirstInteract false)))))

(fn ConstructionScript)

(fn Lock
  (Variables|Default|SetLocked true)
  (Rendering|Material|SetMaterial (Variables|Default|GetbuttonMesh) 0 "/Game/MY_STUFF/Materials/ButtonLocked_MAT.ButtonLocked_MAT"))

(fn Unlock
  (Variables|Default|SetLocked false)
  (Rendering|Material|SetMaterial (Variables|Default|GetbuttonMesh) 0 "/Game/MY_STUFF/Materials/Button_MAT.Button_MAT"))

(fn IsInteractable
  (return (Variables|Default|Getinteractable)))