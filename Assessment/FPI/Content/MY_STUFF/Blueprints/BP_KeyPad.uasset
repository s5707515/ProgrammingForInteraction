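; BP_KeyPad is an interactable keypad that opens a keypad UI and can unlock a linked door.
; OnInteract switches to UI-only input with a visible cursor, then creates UI_Keypad_2 and passes it a self reference.
; The first interaction also changes the objective through BP_ObjectiveManager's UI.
; UnlockDoor opens DoorRef and turns off Interactable, which IsInteractable reports.
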(event EventBeginPlay)

(event Collision|EventActorBeginOverlap
  (params (OtherActor :type Actor%20Object%20Reference)))

(event EventTick
  (params (DeltaSeconds :type Float%20%28single-precision%29)))

(event EventOnInteract
  (bind _returnvalue (Game|GetPlayerController 0))
  (Utilities|FlowControl|Sequence
    (:then_0
      (Input|SetInputModeUIOnly _returnvalue 0 "DoNotLock" true)
      (Variables|/Script/Engine.PlayerController|SetbShowMouseCursor _returnvalue true)
      (Input|SetIgnoreLookInput _returnvalue true)
      (bind _returnvalue_2 (UserInterface|CreateWidget "/Game/MY_STUFF/UI/UI_Keypad_2.UI_Keypad_2_C"))
      (UserInterface|Viewport|AddtoViewport _returnvalue_2 0)
      (Variables|/Game/MY_STUFF/UI/UI_Keypad_2.UI_Keypad_2_C|SetKeyPad%20Ref _returnvalue_2 self))
    (:then_1
      ;[0.15 0.15 0.15 0.5] Update Objective
      (if (Variables|Default|GetfirstInteract)
        (bind _returnvalue_3 (Actor|GetActorOfClass "/Game/MY_STUFF/Blueprints/BP_ObjectiveManager.BP_ObjectiveManager_C"))
        (Class|Objectives|ChangeObjective (Variables|/Game/MY_STUFF/Blueprints/BP_ObjectiveManager.BP_ObjectiveManager_C|GetUI_Ref _returnvalue_3) (Variables|Default|Getobjective))
        (Variables|Default|SetfirstInteract false)))))

(fn ConstructionScript)

(fn UnlockDoor
  (Class|SlidingDoor|OpenDoor (Variables|Default|GetDoor%20Ref))
  (Variables|Default|Setinteractable false))

(fn IsInteractable
  (return (Variables|Default|Getinteractable)))