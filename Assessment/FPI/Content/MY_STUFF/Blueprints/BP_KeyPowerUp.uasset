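; BP_KeyPowerUp is an interactable key pickup that grants the player a key.
; On interact it disables itself, calls AlterNumKeys on the first-person character, and optionally spawns a BP_Platform at a hardcoded world location.
; It then pushes its Objective to the UI through BP_ObjectiveManager and destroys itself.
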(event EventOnInteract
  (Variables|Default|Setinteractable false)
  (bind _returnvalue (Actor|GetActorOfClass "/Game/FirstPerson/Blueprints/BP_FirstPersonCharacter.BP_FirstPersonCharacter_C"))
  (Default|AlterNumKeys _returnvalue 1)
  (if (Variables|Default|GetspawnPlatform)
    (Game|SpawnActorfromClass "/Game/MY_STUFF/Blueprints/BP_Platform.BP_Platform_C" (Math|Transform|MakeTransform "4525.000000,2550.000000,-40.000000") "AlwaysSpawn" "MultiplyWithRoot" 0 0))
  (bind _returnvalue_2 (Actor|GetActorOfClass "/Game/MY_STUFF/Blueprints/BP_ObjectiveManager.BP_ObjectiveManager_C"))
  (Class|Objectives|ChangeObjective (Variables|/Game/MY_STUFF/Blueprints/BP_ObjectiveManager.BP_ObjectiveManager_C|GetUI_Ref _returnvalue_2) (Variables|Default|Getobjective))
  (Actor|DestroyActor))

(fn ConstructionScript)

(fn IsInteractable
  (return (Variables|Default|Getinteractable)))